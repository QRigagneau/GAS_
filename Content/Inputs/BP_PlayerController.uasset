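; Player controller that routes Enhanced Input to the possessed player character for movement, look and shooting.
; BeginPlay adds the default mapping context and caches the controlled pawn as BP_PlayerCharacter.
; Move applies movement along the pawn's right and forward vectors, Look adds controller yaw and pitch, and Shoot calls the cached character's Shoot.
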(event `self.ReceiveBeginPlay`
  (`EnhancedInputSubsystemInterface.AddMappingContext` (subsystem `EnhancedInputLocalPlayerSubsystem`) "/Game/Inputs/IMC_Default.IMC_Default" 0 (make `ModifyContextOptions` true true))
  (bind _asbp_player_character (cast `/Game/Characters/BP_PlayerCharacter` (`self.K2_GetPawn`)))
  (set `self.Control Character` _asbp_player_character))

(event `EnhancedInput|/Game/Inputs/IA_Move`
  (params (ActionValue :type "Vector2D Structure") (ElapsedSeconds :type "Float (double-precision)") (TriggeredSeconds :type "Float (double-precision)") (InputAction :type "InputAction Object Reference" :default "/Game/Inputs/IA_Move.IA_Move"))
  (bind (_x _y) (`KismetMathLibrary.BreakVector2D` ActionValue))
  (bind _returnvalue (`self.K2_GetPawn`))
  (:`Triggered`
    (`Pawn.AddMovementInput` (`self.K2_GetPawn`) (`self.GetActorRightVector` (`self.K2_GetPawn`)) _x false)
    (`Pawn.AddMovementInput` _returnvalue (`self.GetActorForwardVector` _returnvalue) _y false)))

(event `EnhancedInput|/Game/Inputs/IA_Look`
  (params (ActionValue :type "Vector2D Structure") (ElapsedSeconds :type "Float (double-precision)") (TriggeredSeconds :type "Float (double-precision)") (InputAction :type "InputAction Object Reference" :default "/Game/Inputs/IA_Look.IA_Look"))
  (bind (_x _y) (`KismetMathLibrary.BreakVector2D` ActionValue))
  (:`Triggered`
    (`Pawn.AddControllerYawInput` (`self.K2_GetPawn`) _x)
    (`Pawn.AddControllerPitchInput` (`self.K2_GetPawn`) _y)))

(event `EnhancedInput|/Game/Inputs/IA_Shoot`
  (params (ActionValue :type Boolean) (ElapsedSeconds :type "Float (double-precision)") (TriggeredSeconds :type "Float (double-precision)") (InputAction :type "InputAction Object Reference" :default "/Game/Inputs/IA_Shoot.IA_Shoot"))
  (:`Started`
    (`/Game/Characters/BP_PlayerCharacter.Shoot` (`self.Control Character`))))

(fn `UserConstructionScript`)